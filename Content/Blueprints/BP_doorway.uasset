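; BP_doorway is a doorway Blueprint whose door slides open or back when its Interact event fires.
; Interact branches on HasBeenClicked to play or reverse the Lerpinga timeline, which lerps Door1's relative location between DoorStart and DoorStop.
; The construction script clears HasBeenClicked, and the timeline's Update flips it on every tick rather than once per interaction, so the direction of the next Interact depends on the update count.
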(event EventBeginPlay)

(event Collision|EventActorBeginOverlap
  (params (OtherActor :type Actor%20Object%20Reference)))

(event EventTick
  (params (DeltaSeconds :type Float%20%28single-precision%29)))

(event EventInteract
  (if (Variables|Default|Gethas_been_clicked)
    (bind _newtrack_0 (Timeline|lerpinga Reverse)
      (:Update
        (Transformation|SetRelativeLocation (Variables|Default|Getdoor1) (Math|Vector|Lerp(Vector) (Variables|Default|Getdoor%20start) (Variables|Default|Getdoor%20stop) _newtrack_0) false false)
        (Variables|Default|Sethas_been_clicked (not (Variables|Default|Gethas_been_clicked)))))
    (else
      (Timeline|lerpinga Play))))

(fn ConstructionScript
  (Variables|Default|Sethas_been_clicked false))