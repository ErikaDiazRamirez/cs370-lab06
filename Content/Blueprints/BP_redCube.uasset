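; BP_redCube is an interactable cube actor that blends its material when interacted with.
; On BeginPlay it creates a dynamic material instance from ReedMat on the Cube mesh and stores it as BlendInstance.
; Interact prints a red debug string and calls BlendMat, which plays a timeline.
; Each timeline update sets the "blend Value" scalar through the Cube component rather than the stored instance.
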(event Custom|blendMat
  (bind _newtrack_0 (Timeline|Timeline_0 Play)
    (:Update
      (bind _output_get (Variables|Default|SetBlend%20Amount _newtrack_0))
      (Rendering|Material|SetScalarParameterValueonMaterials (Variables|Default|GetCube) "blend Value" _output_get))))

(event Collision|EventActorBeginOverlap
  (params (OtherActor :type Actor%20Object%20Reference)))

(event EventBeginPlay
  (bind _returnvalue (Rendering|Material|CreateDynamicMaterialInstance (Variables|Default|GetCube) 0 "/Game/reedMat.reedMat" "None" :!class /Script/Engine.PrimitiveComponent))
  (Variables|Default|SetblendInstance _returnvalue))

(event EventInteract
  (Development|PrintString "R CUB" true true "(R=1.000000,G=0.239462,B=0.184285,A=1.000000)")
  (CallFunction|BlendMat))

(fn ConstructionScript)