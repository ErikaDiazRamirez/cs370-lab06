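; BP_boo is a Boo-style ghost that creeps toward the player pawn only while off screen.
; Each tick, WasRecentlyRendered either halts it and reverses the Disappear timeline, or moves it at a fixed speed and plays the timeline.
; That timeline drives the BV scalar on the Sphere's dynamic material, created at BeginPlay.
; Its rotation derives from the new position vector rather than the direction to the player.
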(event Collision|EventActorBeginOverlap
  (params (OtherActor :type Actor%20Object%20Reference)))

(event EventTick
  (params (DeltaSeconds :type Float%20%28single-precision%29))
  (bind _returnvalue (Transformation|GetActorLocation))
  (if (Class|Actor|WasRecentlyRendered 0.2)
    (bind _newtrack_0 (Timeline|disappear Reverse)
      (:Update
        (Rendering|Material|SetScalarParameterValueonMaterials (Variables|Default|Getsphere) "BV" _newtrack_0)))
    (else
      (Variables|Default|SetnewNumber 3e+01)
      (Transformation|SetActorLocationAndRotation (+ _returnvalue (* (Variables|Default|GetnewNumber) (* (Math|Vector|Normalize (- (Transformation|GetActorLocation (Game|Player|GetPlayerPawn 0)) _returnvalue)) (Utilities|Time|GetWorldDeltaSeconds)))) (Math|Conversions|RotationFromXVector (+ _returnvalue (* (Variables|Default|GetnewNumber) (* (Math|Vector|Normalize (- (Transformation|GetActorLocation (Game|Player|GetPlayerPawn 0)) _returnvalue)) (Utilities|Time|GetWorldDeltaSeconds))))))
      (Timeline|disappear Play))))

(event EventBeginPlay
  (bind _returnvalue (Rendering|Material|CreateDynamicMaterialInstance (Variables|Default|Getsphere) 0 "/Game/boo_Mat_Inst.boo_Mat_Inst" "None" :!class /Script/Engine.PrimitiveComponent))
  (Variables|Default|SetblendInstanceDynamic _returnvalue))

(fn ConstructionScript)